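; BP_Enemy is an enemy that tracks its distance to the player, takes damage and displays a health widget.
; A looping timer sets one of three State values from distance bands to the player character.
; Damage lowers Health and clears CanTakeDamage until a short timer restores it, though the flag is not checked here.
; Tick smoothly rotates the health widget component to face the player character.
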(event `checkForAggro`
  (bind _returnvalue (`KismetMathLibrary.VSize` (- (`self.K2_GetActorLocation` (`self.target`)) (`self.K2_GetActorLocation`))))
  (if (`KismetMathLibrary.InRange_FloatFloat` _returnvalue 0.0 300.0)
    (set `self.State` "NewEnumerator2")
    (elif (`KismetMathLibrary.InRange_FloatFloat` _returnvalue 300.0 1000.0)
      (set `self.State` "NewEnumerator1")
      (else
        (set `self.State` "NewEnumerator0")))))

(event `self.ReceiveBeginPlay`
  (bind _returnvalue (`|CreateWidget` "/Game/WBP_EnemyHealth.WBP_EnemyHealth_C" null self))
  (`WidgetComponent.SetWidget` (`self.Widget`) _returnvalue)
  (set `self.target` (`GameplayStatics.GetPlayerCharacter` 0))
  (`KismetSystemLibrary.K2_SetTimerDelegate` (delegate `checkForAggro`) 0.5 true))

(event `TakeDamage`
  (params (Damage :type "Float (double-precision)"))
  (set `self.Health` (- (`self.Health`) Damage))
  (set `self.CanTakeDamage` false)
  (`KismetSystemLibrary.K2_SetTimer` null "ResetInvincibility" 0.5))

(event `self.ReceiveTick`
  (params (DeltaSeconds :type "Float (single-precision)"))
  (bind _widget (`self.Widget`))
  (`SceneComponent.K2_SetRelativeRotation` _widget (`KismetMathLibrary.RInterpTo` (`SceneComponent.RelativeRotation` _widget) (`KismetMathLibrary.FindLookAtRotation` (`self.K2_GetActorLocation`) (`self.K2_GetActorLocation` (`GameplayStatics.GetPlayerCharacter` 0))) (`GameplayStatics.GetWorldDeltaSeconds`)) false false))

(fn `ResetInvincibility`
  (set `self.CanTakeDamage` true))

(fn `UserConstructionScript`)