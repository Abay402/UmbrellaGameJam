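; BP_ComboAttack is a combo attack component for the player and enemies, matching accumulated key patterns to montages in AttackData.
; EnterKeyAttack and EnemyAttackKey feed separate DoOnce-gated events that append the key and play the matching montage.
; Completion clears the combo, as does interruption unless another attack montage is active one tick later.
; That interruption check always reads player 0's montage, even on the enemy path.
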(event `AttackCombo`
  (`/Engine/EditorBlueprintResources/StandardMacros.DoOnce` false :!label _label
    (:`Completed`
      (set `self.currentComboPattern` (`KismetStringLibrary.Concat_StrStr` (`self.currentComboPattern`) (`self.currentComboKey`)))
      (for _array_element (`self.attackData`) :!label _label_2
        (bind (_attackanimation _attackpattern) (break `/Game/ComboSystem/Structures/F_ComboAttack` _array_element))
        (if (`KismetStringLibrary.EqualEqual_StrStr` (`self.currentComboPattern`) _attackpattern)
          (`|PlayMontage` (`Character.Mesh` (`GameplayStatics.GetPlayerCharacter` 0)) _attackanimation (`self.animationRate`)
            (:`then`
              (`self.BreakLoop`))
            (:`OnCompleted`
              (set `self.currentComboPattern` "")
              (`self.ResetToNextAttack`)
              (`self.OnAttackAnimationCompleted`))
            (:`OnInterrupted`
              ;[1 1 1] If what interrupted the attack animation is an attack animation defined in the "Attack Data" variable, do not restart the combo. However, if what interrupted the attack animation is any other montage animation (roll, damage, etc.), restart the combo.
              (`KismetSystemLibrary.DelayUntilNextTick`)
              (if (not (`self.CheckIsAttackAnimation`))
                (`self.OnAttackAnimationInterrupted`)
                (set `self.currentComboPattern` "")
                (`self.ResetToNextAttack`)))))))))

(event `ResetToNextAttack`
  (goto _label :!via `Reset`))

(event `BreakLoop`
  (goto _label_2 :!via `Break`))

(event `EnemyAttackCombo`
  (params (Enemy :type "/Game/BP_Enemy Object Reference (by ref)"))
  (`/Engine/EditorBlueprintResources/StandardMacros.DoOnce` false :!label _label_3
    (:`Completed`
      (set `self.currentComboPattern` (`KismetStringLibrary.Concat_StrStr` (`self.currentComboPattern`) (`self.currentComboKey`)))
      (for _array_element (`self.attackData`) :!label _label_4
        (bind (_attackanimation _attackpattern) (break `/Game/ComboSystem/Structures/F_ComboAttack` _array_element))
        (if (`KismetStringLibrary.EqualEqual_StrStr` (`self.currentComboPattern`) _attackpattern)
          (`|PlayMontage` (`Character.Mesh` Enemy) _attackanimation (`self.animationRate`)
            (:`then`
              (`self.Break`))
            (:`OnCompleted`
              (set `self.currentComboPattern` "")
              (`self.ResetAttack`)
              (`self.OnAttackAnimationCompleted`))
            (:`OnInterrupted`
              ;[1 1 1] If what interrupted the attack animation is an attack animation defined in the "Attack Data" variable, do not restart the combo. However, if what interrupted the attack animation is any other montage animation (roll, damage, etc.), restart the combo.
              (`KismetSystemLibrary.DelayUntilNextTick`)
              (if (not (`self.CheckIsAttackAnimation`))
                (`self.OnAttackAnimationInterrupted`)
                (set `self.currentComboPattern` "")
                (`self.ResetAttack`)))))))))

(event `ResetAttack`
  (goto _label_3 :!via `Reset`))

(event `Break`
  (goto _label_4 :!via `Break`))

(fn `CheckIsAttackAnimation`
  (returns (ReturnValue :type Boolean))
  (locals (attackAnimations :type "Array of AnimMontage Object Reference"))
  (for _array_element (`self.attackData`)
    (`KismetArrayLibrary.Array_AddUnique` (`local.attackAnimations`) (`.attackAnimation_5_4D5CC6AA41565397ACEAECBE047327A8` (break `/Game/ComboSystem/Structures/F_ComboAttack` _array_element))))
  (return (`KismetArrayLibrary.Array_Contains` (`local.attackAnimations`) (`AnimInstance.GetCurrentActiveMontage` (`SkeletalMeshComponent.GetAnimInstance` (`Character.Mesh` (`GameplayStatics.GetPlayerCharacter` 0)))))))

(fn `EnemyAttackKey`
  (params (Key :type String) (Enemy :type "/Game/BP_Enemy Object Reference"))
  (set `self.currentComboKey` Key)
  (`self.EnemyAttackCombo` Enemy)
  (return))

(fn `EnterKeyAttack`
  (params (key :type String))
  (set `self.currentComboKey` key)
  (`self.AttackCombo`)
  (return))